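; Animation group for the princess character that gathers several Creature animation actors into one named clip collection.
; On BeginPlay, it casts four child actor components to CreatureActor and registers their clips by name.
; The clips cover ground stand and walk, jump start, air rise and fall, and landing, with some actors supplying two clips.
; The Blueprint only registers clips and contains no playback or switching logic.
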(event `self.ReceiveBeginPlay`
  (`|ExecutionSequence`
    (:`then_0`
      (bind _ascreature_actor (cast `CreatureActor` (`ChildActorComponent.ChildActor` (`self.GroundStand`))))
      (`self.AddBluePrintCollectionClipData` "ground_stand" _ascreature_actor "ground_stand")
      (`self.AddBluePrintCollectionClipData` "ground_walk" _ascreature_actor "ground_walk"))
    (:`then_1`
      (bind _ascreature_actor_2 (cast `CreatureActor` (`ChildActorComponent.ChildActor` (`self.GroundStartJump`))))
      (`self.AddBluePrintCollectionClipData` "ground_start_jump" _ascreature_actor_2 "ground_start_jump"))
    (:`then_2`
      (bind _ascreature_actor_3 (cast `CreatureActor` (`ChildActorComponent.ChildActor` (`self.AirJumpUp`))))
      (`self.AddBluePrintCollectionClipData` "air_jump_up" _ascreature_actor_3 "air_jump_up"))
    (:`then_3`
      (bind _ascreature_actor_4 (cast `CreatureActor` (`ChildActorComponent.ChildActor` (`self.AirJumpDown`))))
      (`self.AddBluePrintCollectionClipData` "air_jump_down" _ascreature_actor_4 "air_jump_down")
      (`self.AddBluePrintCollectionClipData` "ground_end_jump" _ascreature_actor_4 "ground_end_jump"))))

(event `self.ReceiveActorBeginOverlap`
  (params (OtherActor :type "Actor Object Reference")))

(event `self.ReceiveTick`
  (params (DeltaSeconds :type "Float (single-precision)")))

(fn `UserConstructionScript`)