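; BP_Princess is a side-scrolling player character that walks along the X axis and supports limited multi-jumps.
; Movement, jump and touch input drive animation states on a child-actor humanoid animation collection, with facing flipped through control yaw.
; Jump input starts the animation first; a separate real-start event then launches the jump, sets horizontal velocity from input and cuts it short if released.
; Apex, landing and ledge events update animation, and landing resets the jump count.
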(event `self.ReceiveBeginPlay`
  ;[1 1 1] 初始化和消息绑定
  (bind _asbp_humanoid_animation (cast `/Game/ProjectC/Blueprints/CreatureCollection/BP_HumanoidAnimation` (`ChildActorComponent.ChildActor` (`self.AniCreatureCollection`))))
  (set `self.CurAnimationCollection` _asbp_humanoid_animation)
  (`|ExecutionSequence`
    (:`then_0`
      (add `/Game/ProjectC/Blueprints/CreatureCollection/BP_HumanoidAnimation.OnJumpReadyEnd` (`self.CurAnimationCollection`) (`|CreateDelegate` self :!event `OnJumpRealStart`)))
    (:`then_1`
      (add `self.OnReachedJumpApex` (`|CreateDelegate` self :!event `OnJumpApex`)))
    (:`then_2`
      (add `self.OnTurnRound` (`|CreateDelegate` (`self.PlatformCameraSpring`) :!event `OnTurnRound`))
      (set `self.CurForwardVector` (`SceneComponent.GetForwardVector` (`self.CapsuleComponent`))))))

(event `self.ReceiveTick`
  (params (DeltaSeconds :type "Float (single-precision)"))
  ;[0.1339 0.5481 1] 帧更新消息
)

(event `InputAction|Jump`
  ;[1 0.9811 0.434] 跳跃消息
  (:`Pressed`
    (set `self.IsJumpPressed` true :!label _label)
    (if (`self.CheckCamInputJump`)
      (`/Game/ProjectC/Blueprints/CreatureCollection/BP_HumanoidAnimation.OnActionJump` (`self.CurAnimationCollection`))))
  (:`Released`
    (set `self.IsJumpPressed` false :!label _label_2)))

(event `InputAxis|MoveRight`
  (params (AxisValue :type "Float (single-precision)"))
  (bind _curanimationcollection (`self.CurAnimationCollection`))
  (bind _returnvalue (`KismetMathLibrary.Normal` (`self.GetVelocity`)))
  ;[0.4064 1 0.4323] 移动消息
  (set `self.CurInputAxis` AxisValue)
  (`self.AddMovementInput` (1.0 0.0 0.0) AxisValue)
  (`/Engine/EditorBlueprintResources/StandardMacros.CompareFloat` AxisValue
    (:`>`
      (`Controller.SetControlRotation` (`self.GetController`) (`KismetMathLibrary.MakeRot` 0.0 0.0))
      (`/Game/ProjectC/Blueprints/CreatureCollection/BP_HumanoidAnimation.OnStartWalk` _curanimationcollection :!label _label_3)
      (if (!= (`self.CurForwardVector`) _returnvalue)
        (bind _output_get (set `self.CurForwardVector` _returnvalue))
        (`self.OnTurnRound` _output_get)))
    (:`==`
      (`/Game/ProjectC/Blueprints/CreatureCollection/BP_HumanoidAnimation.OnStartStand` _curanimationcollection))
    (:`<`
      (`Controller.SetControlRotation` (`self.GetController`) (`KismetMathLibrary.MakeRot` 0.0 180.0))
      (goto _label_3))))

(event `InputTouch`
  (params (Location :type "Vector Structure") (FingerIndex :type "ETouchIndex Enum"))
  ;[1 0.9811 0.434] 跳跃消息
  (:`Pressed`
    (goto _label))
  (:`Released`
    (goto _label_2)))

(event `OnJumpRealStart`
  (bind _charactermovement (`self.CharacterMovement`))
  (bind _jumpinitialspeedx (`self.JumpInitialSpeedX`))
  ;[1 0.9811 0.434] 跳跃消息
  (`self.Jump`)
  (`|ExecutionSequence`
    (:`then_0`
      (set `CharacterMovementComponent.bNotifyApex` true (`self.CharacterMovement`))
      (set `self.CurJumpCount` (+ (`self.CurJumpCount`) 1))
      (`/Engine/EditorBlueprintResources/StandardMacros.CompareFloat` (`self.CurInputAxis`)
        (:`>`
          (set `MovementComponent.Velocity` (`KismetMathLibrary.MakeVector` _jumpinitialspeedx) _charactermovement))
        (:`==`
          (set `MovementComponent.Velocity` (0.0 0.0 0.0) _charactermovement))
        (:`<`
          (set `MovementComponent.Velocity` (`KismetMathLibrary.MakeVector` (* _jumpinitialspeedx -1.0)) _charactermovement))))
    (:`then_1`
      (if (not (`self.IsJumpPressed`))
        (`KismetSystemLibrary.Delay` 0.01)
        (`self.StopJumping`)))))

(event `OnJumpApex`
  ;[1 0.9811 0.434] 跳跃消息
  (`/Game/ProjectC/Blueprints/CreatureCollection/BP_HumanoidAnimation.OnJumpApex` (`self.CurAnimationCollection`)))

(event `self.OnLanded`
  (params (Hit :type "HitResult Structure (by ref)"))
  ;[1 0.9811 0.434] 跳跃消息
  (`/Game/ProjectC/Blueprints/CreatureCollection/BP_HumanoidAnimation.OnLanded` (`self.CurAnimationCollection`))
  (set `self.CurJumpCount` 0))

(event `OnJumpToStand`
  ;[1 0.9811 0.434] 跳跃消息
)

(event `self.OnWalkingOffLedge`
  (params (PreviousFloorImpactNormal :type "Vector Structure (by ref)") (PreviousFloorContactNormal :type "Vector Structure (by ref)") (PreviousLocation :type "Vector Structure (by ref)") (TimeDelta :type "Float (single-precision)"))
  ;[1 0.9811 0.434] 跳跃消息
  (`/Game/ProjectC/Blueprints/CreatureCollection/BP_HumanoidAnimation.OnStartFall` (`self.CurAnimationCollection`)))

(fn `CanJumpInternal`
  (returns (ReturnValue :type Boolean))
  (bind _returnvalue (`parent.CanJumpInternal`))
  (return (and (or _returnvalue (`NavMovementComponent.IsFalling` (`self.CharacterMovement`))) (not (`self.CheckJumpCountLimit`)))))

(fn `CheckCamInputJump`
  (returns (CanInputJump :type Boolean))
  (return (< (`self.CurJumpCount`) (`self.JumpMaxCount`))))

(fn `CheckJumpCountLimit`
  (returns (IsLimit :type Boolean))
  (return (not (<= (`self.CurJumpCount`) (`self.JumpMaxCount`)))))

(fn `UserConstructionScript`)