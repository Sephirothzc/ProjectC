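; BP_TestCollection is a test pawn that hosts a CreatureCollectionActor through a child actor and moves along world X with MoveRight input.
; BeginPlay caches that actor and starts its "ground_stand" clip looping.
; MoveRight sets an animation state, flipping control yaw between 0 and 180 when on ground.
; That state never reaches the creature: UpdateAnimation is empty and the clip-switching nodes are unconnected.
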(event `UpdateAnimation`)

(event `self.ReceiveBeginPlay`
  (bind _ascreature_collection_actor (cast `CreatureCollectionActor` (`ChildActorComponent.ChildActor` (`self.ChildActor`))))
  (bind _output_get (set `self.CurCreateGroup` _ascreature_collection_actor))
  (`CreatureCollectionActor.SetBluePrintShouldPlay` _output_get true)
  (`CreatureCollectionActor.SetBluePrintIsLooping` _output_get true)
  (`CreatureCollectionActor.SetBluePrintActiveClip` _output_get "ground_stand"))

(event `self.ReceiveActorBeginOverlap`
  (params (OtherActor :type "Actor Object Reference")))

(event `self.ReceiveTick`
  (params (DeltaSeconds :type "Float (single-precision)")))

(event `InputAxis|MoveRight`
  (params (AxisValue :type "Float (single-precision)"))
  (bind _curgameobjstate (`self.CurGameObjState`))
  (`self.AddMovementInput` (1.0 0.0 0.0) AxisValue)
  (`/Engine/EditorBlueprintResources/StandardMacros.CompareFloat` AxisValue
    (:`>`
      (`|ExecutionSequence`
        (:`then_0`
          (switch `/Game/ProjectC/Blueprints/E_GameObjState` _curgameobjstate
            (:`NewEnumerator0`
              (`Controller.SetControlRotation` (`self.GetController`) (`KismetMathLibrary.MakeRot` 0.0 0.0)))))
        (:`then_1`
          (set `self.CurAnimationState` "NewEnumerator1" :!label _label))))
    (:`==`
      (switch `/Game/ProjectC/Blueprints/E_GameObjState` _curgameobjstate
        (:`NewEnumerator0`
          (set `self.CurAnimationState` "NewEnumerator0"))))
    (:`<`
      (`|ExecutionSequence`
        (:`then_0`
          (switch `/Game/ProjectC/Blueprints/E_GameObjState` _curgameobjstate
            (:`NewEnumerator0`
              (`Controller.SetControlRotation` (`self.GetController`) (`KismetMathLibrary.MakeRot` 0.0 180.0))
              (goto _label))))
        (:`then_1`
          (goto _label))))))

(fn `UserConstructionScript`)