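; Parent Blueprint for animation groups that gathers Creature actors under shared animation names.
; On BeginPlay it matches each AnimationList entry to "CreatureUnit"-tagged child actor components by object name and casts their child actors to CreatureActor.
; Each match registers a collection clip mapping the group name to the creature's clip, and adds an AnimationCreatureMap node with an empty creature animation name.
; ChangeAnimationTo is an empty stub.
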(event `self.ReceiveBeginPlay`
  (for _array_element (`self.AnimationList`)
    (for _array_element_2 (`self.GetComponentsByTag` "/Script/Engine.ChildActorComponent" "CreatureUnit")
      (bind (_realanimationname _animationinstance) (break `/Game/ProjectC/Blueprints/S_AnimationCollection` _array_element))
      (bind (_creaturename _animationname) (break `/Game/ProjectC/Blueprints/S_AnimationClip` _animationinstance))
      (if (`KismetStringLibrary.EqualEqual_StrStr` (`KismetSystemLibrary.GetObjectName` _array_element_2) _creaturename)
        (bind _ascreature_actor (cast `CreatureActor` (`ChildActorComponent.ChildActor` _array_element_2)))
        (`self.AddBluePrintCollectionClipData` _realanimationname _ascreature_actor _animationname)
        (`KismetArrayLibrary.Array_Add` (`self.AnimationCreatureMap`) (make `/Game/ProjectC/Blueprints/S_AnimationCreatureMapNode` _realanimationname _ascreature_actor))))))

(event `self.ReceiveActorBeginOverlap`
  (params (OtherActor :type "Actor Object Reference")))

(event `self.ReceiveTick`
  (params (DeltaSeconds :type "Float (single-precision)")))

(fn `ChangeAnimationTo`
  (params (NextAnimation :type String)))

(fn `UserConstructionScript`)