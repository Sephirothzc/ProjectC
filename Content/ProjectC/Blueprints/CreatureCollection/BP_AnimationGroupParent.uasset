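; BP_AnimationGroupParent is a Creature animation collection base that groups several CreatureActors by animation.
; InitCollection matches each AnimationList entry's creature name against child actor components tagged "CreatureUnit".
; Matched actors get a collection clip named from the animation enum and are recorded in AnimationCreatureMap.
; Any name mismatch or failed cast sets IsSuccess false, even if another component matches.
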(fn ConstructionScript)

(fn InitCollection
  (for _array_element (Variables|CreatureCollection|GetAnimationList)
    (for _array_element_2 (Actor|GetComponentsbyTag "/Script/Engine.ChildActorComponent" "CreatureUnit")
      (if (Utilities|Enum|Equal(Enum) (Utilities|GetObjectName _array_element_2) (.CreatureName (Utilities|Struct|BreakS_AnimationCollection _array_element)))
        (bind _ascreature_actor (Utilities|Casting|CastToCreatureActor (Variables|/Script/Engine.ChildActorComponent|GetChildActor _array_element_2))
          (:then
            (Class|CreatureCollectionActor|AddBluePrintCollectionClipData (Utilities|String|EnumtoString (.AnimationName (Utilities|Struct|BreakS_AnimationCollection _array_element))) _ascreature_actor (Utilities|String|EnumtoString (.AnimationName (Utilities|Struct|BreakS_AnimationCollection _array_element))))
            (Utilities|Array|Add (Variables|CreatureCollection|GetAnimationCreatureMap) (Utilities|Struct|MakeS_AnimationCreatureMapNode (.AnimationName (Utilities|Struct|BreakS_AnimationCollection _array_element)) _ascreature_actor)))
          (:CastFailed
            (LocalVariables|SetIsSuccess false)))
        (else
          (LocalVariables|SetIsSuccess false)))))
  (return (LocalVariables|GetIsSuccess)))