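; BP_HumanoidAnimation is a humanoid animation state machine that starts in the ground-stand state.
; InitCollection gives each BP_HumanoidAniState component tagged AniState a back-reference to itself.
; Movement, jump, fall, landing and attack events forward to the current state object, following the State pattern.
; ChangeAniState exits the current state and enters the next one when it is valid.
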(event `self.ReceiveBeginPlay`
  (`parent.ReceiveBeginPlay`)
  (`self.InitCollection`)
  (`self.ChangeAniState` (`self.HumanoidAniState_GroundStand`)))

(event `OnStartWalk`
  (`/Game/ProjectC/Blueprints/CreatureCollection/HumanoidAniState/IBP_HumanoidAniState.OnStartWalk` (`self.CurAniState`)))

(event `OnStartStand`
  (`/Game/ProjectC/Blueprints/CreatureCollection/HumanoidAniState/IBP_HumanoidAniState.OnStartStand` (`self.CurAniState`)))

(event `OnActionJump`
  (`/Game/ProjectC/Blueprints/CreatureCollection/HumanoidAniState/IBP_HumanoidAniState.OnActionJump` (`self.CurAniState`)))

(event `OnJumpApex`
  (`/Game/ProjectC/Blueprints/CreatureCollection/HumanoidAniState/IBP_HumanoidAniState.OnJumpApex` (`self.CurAniState`)))

(event `OnLanded`
  (`/Game/ProjectC/Blueprints/CreatureCollection/HumanoidAniState/IBP_HumanoidAniState.OnLanded` (`self.CurAniState`)))

(event `OnStartFall`
  (`/Game/ProjectC/Blueprints/CreatureCollection/HumanoidAniState/IBP_HumanoidAniState.OnStartFall` (`self.CurAniState`)))

(event `OnAttackKey1Down`
  (`/Game/ProjectC/Blueprints/CreatureCollection/HumanoidAniState/IBP_HumanoidAniState.OnAttackKey1Down` (`self.CurAniState`)))

(fn `ChangeAniState`
  (params (NextAniState :type "/Game/ProjectC/Blueprints/CreatureCollection/HumanoidAniState/BP_HumanoidAniState Object Reference (by ref)"))
  (`/Engine/EditorBlueprintResources/StandardMacros.IsValid` NextAniState
    (:`Is Valid`
      (`/Engine/EditorBlueprintResources/StandardMacros.IsValid` (`self.CurAniState`)
        (:`Is Valid`
          (`CreatureAniState.ExitState` (`self.CurAniState`)))
        (:`Is Not Valid`
          _))
      (`CreatureAniState.EnterState` NextAniState)
      (set `self.CurAniState` NextAniState))))

(fn `InitCollection`
  (returns (NewParam :type Boolean))
  (`parent.InitCollection`)
  (for _array_element (`self.GetComponentsByTag` "/Game/ProjectC/Blueprints/CreatureCollection/HumanoidAniState/BP_HumanoidAniState.BP_HumanoidAniState_C" "AniState")
    (set `/Game/ProjectC/Blueprints/CreatureCollection/HumanoidAniState/BP_HumanoidAniState.ParentAni` self _array_element))
  (return false))

(fn `UserConstructionScript`
  (`parent.UserConstructionScript`))