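; BP_HumanoidAniState is an animation state for humanoid Creature animations, with enter, update and exit functions.
; EnterState sets looping on ParentAni and activates the clip named by the CurAniName enum, converted to a string.
; UpdateState and ExitState only return true.
; Separate functions bind and unbind a delegate to ParentAni's animation-end event.
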(fn `BindAnimationEndEvent`
  (add `CreatureCollectionActor.CreatureAnimationEndEvent` (`self.ParentAni`) (`|CreateDelegate` self :!event `OnAnimationEnd`)))

(fn `EnterState`
  (returns (ReturnValue :type Boolean))
  (bind _parentani (`self.ParentAni`))
  (`CreatureCollectionActor.SetBluePrintIsLooping` _parentani (`self.IsAnimationLoop`))
  (`CreatureCollectionActor.SetBluePrintActiveClip` _parentani (`|GetEnumeratorNameAsString` (`self.CurAniName`)))
  (return true))

(fn `ExitState`
  (returns (ReturnValue :type Boolean))
  (return true))

(fn `UnbindAnimationEndEvent`
  (remove `CreatureCollectionActor.CreatureAnimationEndEvent` (`self.ParentAni`) (`|CreateDelegate` self :!event `OnAnimationEnd`)))

(fn `UpdateState`
  (params (delta_seconds :type "Float (double-precision)"))
  (returns (ReturnValue :type Boolean))
  (return true))