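; Parent Blueprint for humanoid animation groups that combine several Creature actors into one clip collection with switchable animation states.
; InitCollection matches AnimationList entries to "CreatureUnit"-tagged child actor components by object name, then registers their clips and records them in AnimationCreatureMap.
; ChangeAnimationTo runs can-change, exit and enter hook functions, storing the result as CurAnimationState.
; These hooks are pass-through defaults that allow every change and play nothing themselves.
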(event `self.ReceiveActorBeginOverlap`
  (params (OtherActor :type "Actor Object Reference")))

(event `self.ReceiveTick`
  (params (DeltaSeconds :type "Float (single-precision)")))

(fn `CanChangeStateFunc`
  (params (CurStateName :type "/Game/ProjectC/Blueprints/Enumerate/E_HumanoidAnimationState Enum") (NextStateName :type "/Game/ProjectC/Blueprints/Enumerate/E_HumanoidAnimationState Enum"))
  (returns (CanChange :type Boolean))
  (return true))

(fn `ChangeAnimationTo`
  (params (NextAnimation :type "/Game/ProjectC/Blueprints/Enumerate/E_HumanoidAnimationState Enum") (IsLoop :type Boolean))
  (returns (IsSuccess :type Boolean))
  (bind _canchange (`self.CanChangeStateFunc` (`self.CurAnimationState`) NextAnimation))
  (if _canchange
    (`|ExecutionSequence`
      (:`then_0`
        (`self.OnStateExitFunc` (`self.CurAnimationState`)))
      (:`then_1`
        (bind _nextstate (`self.OnStateEnterFunc` NextAnimation IsLoop))
        (set `self.CurAnimationState` _nextstate)
        (return _canchange)))
    (else
      (return _canchange))))

(fn `InitCollection`
  (for _array_element (`self.AnimationList`)
    (for _array_element_2 (`self.GetComponentsByTag` "/Script/Engine.ChildActorComponent" "CreatureUnit")
      (bind (_realanimationname _creaturename _animationname) (break `/Game/ProjectC/Blueprints/Structure/S_AnimationCollection` _array_element))
      (if (`KismetStringLibrary.EqualEqual_StrStr` (`KismetSystemLibrary.GetObjectName` _array_element_2) _creaturename)
        (bind _ascreature_actor (cast `CreatureActor` (`ChildActorComponent.ChildActor` _array_element_2)))
        (`self.AddBluePrintCollectionClipData` _realanimationname _ascreature_actor _animationname)
        (`KismetArrayLibrary.Array_Add` (`self.AnimationCreatureMap`) (make `/Game/ProjectC/Blueprints/Structure/S_AnimationCreatureMapNode` _realanimationname _ascreature_actor _animationname))))))

(fn `OnStateEnterFunc`
  (params (NextStateName :type "/Game/ProjectC/Blueprints/Enumerate/E_HumanoidAnimationState Enum") (IsLoop :type Boolean))
  (returns (NextState :type "/Game/ProjectC/Blueprints/Enumerate/E_HumanoidAnimationState Enum"))
  (return NextStateName))

(fn `OnStateExitFunc`
  (params (CurStateName :type "/Game/ProjectC/Blueprints/Enumerate/E_HumanoidAnimationState Enum"))
  (returns (CurState :type "/Game/ProjectC/Blueprints/Enumerate/E_HumanoidAnimationState Enum"))
  (return CurStateName))

(fn `UserConstructionScript`)