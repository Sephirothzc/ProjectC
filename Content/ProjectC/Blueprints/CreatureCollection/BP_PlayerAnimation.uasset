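; BP_PlayerAnimation is a creature-collection actor that, by its name, manages player animation through a component-based state machine.
; InitCollection extends the parent version by setting itself as ParentAni on every BP_HumanoidAniState component tagged "AniState".
; ChangeAniState exits the current state if valid, enters the requested one and stores it as current.
; The event graph adds no behavior of its own.
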(event `self.ReceiveBeginPlay`
  (`parent.ReceiveBeginPlay`))

(event `self.ReceiveActorBeginOverlap`
  (params (OtherActor :type "Actor Object Reference")))

(event `self.ReceiveTick`
  (params (DeltaSeconds :type "Float (single-precision)")))

(fn `ChangeAniState`
  (params (NextAniState :type "/Game/ProjectC/Blueprints/CreatureCollection/HumanoidAniState/BP_HumanoidAniState Object Reference"))
  (`/Engine/EditorBlueprintResources/StandardMacros.IsValid` (`self.CurAniState`)
    (:`Is Valid`
      (`CreatureAniState.ExitState` (`self.CurAniState`)))
    (:`Is Not Valid`
      _))
  (`CreatureAniState.EnterState` NextAniState)
  (set `self.CurAniState` NextAniState))

(fn `InitCollection`
  (returns (NewParam :type Boolean))
  (bind _newparam (`parent.InitCollection`))
  (for _array_element (`self.GetComponentsByTag` "/Game/ProjectC/Blueprints/CreatureCollection/HumanoidAniState/BP_HumanoidAniState.BP_HumanoidAniState_C" "AniState")
    (set `/Game/ProjectC/Blueprints/CreatureCollection/HumanoidAniState/BP_HumanoidAniState.ParentAni` self _array_element))
  (return _newparam))

(fn `UserConstructionScript`
  (`parent.UserConstructionScript`))