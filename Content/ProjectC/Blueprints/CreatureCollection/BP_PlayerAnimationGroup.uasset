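; Player animation state machine that switches Creature clips for standing, walking, jumping and falling.
; Each update requests walk or stand from velocity, or the fall clip when airborne outside a jump.
; Jump events chain clips through animation-end callbacks and notify listeners when takeoff and landing finish.
; Overridden parent hooks whitelist transitions per state and activate the clip named after the entered enum state.
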(event Custom|OnFallEnd
  ;[0.8965 1 0.5412] 跳跃消息
  (bind _issuccess (CallFunction|ChangeAnimationto "NewEnumerator3" false))
  (if _issuccess
    (EventDispatchers|BindEventtoCreatureAnimationEndEvent (delegate Custom|OnEndJump))))

(event Custom|OnStartJump
  ;[0.8965 1 0.5412] 跳跃消息
  (bind _issuccess (CallFunction|ChangeAnimationto "NewEnumerator2" false))
  (if _issuccess
    (EventDispatchers|BindEventtoCreatureAnimationEndEvent (delegate Custom|OnRealStartJump))
    (Variables|Default|SetIsJumpProcess true)))

(event Custom|OnStartJumpFall
  ;[0.8965 1 0.5412] 跳跃消息
  (CallFunction|ChangeAnimationto "NewEnumerator5" true))

(event Custom|OnRealStartJump
  (params (frame :type Float%20%28single-precision%29))
  ;[0.8965 1 0.5412] 跳跃消息
  (bind _issuccess (CallFunction|ChangeAnimationto "NewEnumerator4" true))
  (if _issuccess
    (EventDispatchers|UnbindEventfromCreatureAnimationEndEvent (delegate Custom|OnRealStartJump))
    (Default|CallOnJumpReadyEnd)))

(event Custom|UpdateAnimation
  (params (Delta%20Seconds :type Float%20%28single-precision%29))
  ;[0 0.4249 1] 动画更新消息
  (if (and (Variables|Default|GetIsAir) (not (Variables|Default|GetIsJumpProcess)))
    (CallFunction|ChangeAnimationto "NewEnumerator5" true)
    (elif (> (Math|Vector|VectorLength (Variables|Default|GetCurVelcoity)) 0.0)
      (CallFunction|ChangeAnimationto "NewEnumerator1" true)
      (else
        (CallFunction|ChangeAnimationto "NewEnumerator0" true)))))

(event Custom|OnEndJump
  (params (frame :type Float%20%28single-precision%29))
  ;[0.8965 1 0.5412] 跳跃消息
  (bind _issuccess (CallFunction|ChangeAnimationto "NewEnumerator0" false))
  (if _issuccess
    (EventDispatchers|UnbindEventfromCreatureAnimationEndEvent (delegate Custom|OnEndJump))
    (Default|CallOnJumpAllEnd)
    (Variables|Default|SetIsJumpProcess false)))

(event EventBeginPlay
  ;[1 1 1] 初始化
  (|CallParentFunction)
  (CallFunction|InitCollection)
  (CallFunction|ChangeAnimationto "NewEnumerator0" true))

(fn ConstructionScript
  (|CallParentFunction))

(fn CanChangeStateFunc
  (params (CurStateName :type E_HumanoidAnimationState%20Enum :default "NewEnumerator7") (NextStateName :type E_HumanoidAnimationState%20Enum :default "NewEnumerator7"))
  (bind _canchange (|CallParentFunction CurStateName NextStateName))
  (LocalVariables|SetLocalNextState NextStateName)
  (LocalVariables|SetParentReturnValue _canchange)
  (switch Utilities|FlowControl|Switch|SwitchonE_HumanoidAnimationState CurStateName
    (:NewEnumerator7
      (bind _checkresult (|CheckNoneState (LocalVariables|GetLocalNextState)))
      (LocalVariables|SetReturnValue (and (LocalVariables|GetParentReturnValue) _checkresult)))
    (:NewEnumerator0
      (bind _checkresult_2 (|CheckGroundStand (LocalVariables|GetLocalNextState)))
      (LocalVariables|SetReturnValue (and (LocalVariables|GetParentReturnValue) _checkresult_2)))
    (:NewEnumerator1
      (bind _checkresult_3 (|CheckGroundWalk (LocalVariables|GetLocalNextState)))
      (LocalVariables|SetReturnValue (and (LocalVariables|GetParentReturnValue) _checkresult_3)))
    (:NewEnumerator2
      (bind _checkresult_4 (|CheckStartJump (LocalVariables|GetLocalNextState)))
      (LocalVariables|SetReturnValue (and (LocalVariables|GetParentReturnValue) _checkresult_4)))
    (:NewEnumerator3
      (bind _checkresult_5 (|CheckEndJump (LocalVariables|GetLocalNextState)))
      (LocalVariables|SetReturnValue (and (LocalVariables|GetParentReturnValue) _checkresult_5)))
    (:NewEnumerator4
      (bind _checkresult_6 (|CheckAirJumpUp (LocalVariables|GetLocalNextState)))
      (LocalVariables|SetReturnValue (and (LocalVariables|GetParentReturnValue) _checkresult_6)))
    (:NewEnumerator5
      (bind _checkresult_7 (|CheckJumpDown (LocalVariables|GetLocalNextState)))
      (LocalVariables|SetReturnValue (and (LocalVariables|GetParentReturnValue) _checkresult_7))))
  (return (LocalVariables|GetReturnValue)))

(fn OnStateEnterFunc
  (params (NextStateName :type E_HumanoidAnimationState%20Enum :default "NewEnumerator7") (IsLoop :type Boolean))
  (bind _nextstate (|CallParentFunction NextStateName IsLoop))
  (switch Utilities|FlowControl|Switch|SwitchonE_HumanoidAnimationState _nextstate
    (:NewEnumerator7
      (Development|PrintString "error state"))
    (:NewEnumerator0
      (Class|CreatureCollectionActor|SetBluePrintActiveClip (Utilities|String|EnumtoString _nextstate) :!label _label))
    (:NewEnumerator1
      (goto _label))
    (:NewEnumerator2
      (goto _label))
    (:NewEnumerator3
      (goto _label))
    (:NewEnumerator4
      (goto _label))
    (:NewEnumerator5
      (goto _label)))
  (return _nextstate))

(fn OnStateExitFunc
  (params (CurStateName :type E_HumanoidAnimationState%20Enum :default "NewEnumerator7"))
  (bind _curstate (|CallParentFunction CurStateName))
  (switch Utilities|FlowControl|Switch|SwitchonE_HumanoidAnimationState _curstate
    (:NewEnumerator7
      _)
    (:NewEnumerator0
      _)
    (:NewEnumerator1
      _)
    (:NewEnumerator2
      _)
    (:NewEnumerator3
      _)
    (:NewEnumerator4
      _)
    (:NewEnumerator5
      _))
  (return _curstate))

(fn SetVelcoity
  (params (Velcoity :type Vector))
  (Variables|Default|SetCurVelcoity Velcoity))

(fn SetIsAir
  (params (IsAir :type Boolean))
  (Variables|Default|SetIsAir IsAir))