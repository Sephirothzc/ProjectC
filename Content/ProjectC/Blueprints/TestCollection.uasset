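; Test Blueprint for a creature clip collection that plays animation clips on two child CreatureActors together.
; BeginPlay registers a ground jump-start and an air jump-up clip under one looping collection clip, then sizes a timeline by its frame count.
; Tick detects changes in the clip's current frame to reset the timeline's time, and a timeline event prints a debug "start end" message.
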(event `self.ReceiveBeginPlay`
  (`|ExecutionSequence`
    (:`then_0`
      (bind _ascreature_actor (cast `CreatureActor` (`ChildActorComponent.ChildActor` (`self.ChildActor`))))
      (`self.AddBluePrintCollectionClipData` "test1" _ascreature_actor "ground_start_jump")
      (bind _ascreature_actor_2 (cast `CreatureActor` (`ChildActorComponent.ChildActor` (`self.ChildActor1`))))
      (`self.AddBluePrintCollectionClipData` "test1" _ascreature_actor_2 "air_jump_up")
      (`self.SetBluePrintActiveClip` "test1")
      (`self.SetBluePrintIsLooping` true)
      (`TimelineComponent.SetTimelineLength` (`self.Timeline_0`) (`self.GetBluePrintClipTotalFrames` "test1")))
    (:`then_1`
      (`Timeline|Timeline_0` :`NewTime` (`self.GetBluePrintClipCurFrames` "test1") :!label _label
        (:`startEnd`
          (`KismetSystemLibrary.PrintString` "start end"))))))

(event `self.ReceiveActorBeginOverlap`
  (params (OtherActor :type "Actor Object Reference")))

(event `self.ReceiveTick`
  (params (DeltaSeconds :type "Float (single-precision)"))
  (bind _returnvalue (`self.GetBluePrintClipCurFrames` "test1"))
  (if (!= (`self.PreFrame`) _returnvalue)
    (set `self.PreFrame` _returnvalue)
    (goto _label :!via `SetNewTime`)))

(fn `UserConstructionScript`)